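; BP_NestElvis2 is a nest Blueprint that moves BPFatElvis in alternating bursts of motion and pauses.
; StartMoving sets its Speed and plays Timeline2 from the start, while function-name timers alternate StopMoving after TimeAction and ContinueMoving after TimeOpposition.
; Stopping zeroes Speed and halts the timeline, which resumes where it left off.
; Timeline updates feed MoveTurtle, and completion zeroes Speed and calls ResetActivation.
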(event `ContinueMoving`
  (set `/Game/Character/BP_FatElvis.Speed` (`self.Speed`) (`self.BP_FatElvis`))
  (`KismetSystemLibrary.K2_SetTimer` null "StopMoving" (`self.TimeAction`))
  (bind (_direction _time) (`Timeline|Timeline2` :!label _label)
    (:`Update`
      (`self.MoveTurtle` _time))
    (:`Finished`
      (set `/Game/Character/BP_FatElvis.Speed` 0.0 (`self.BP_FatElvis`))
      (`self.ResetActivation`))))

(event `self.StartMoving`
  (set `/Game/Character/BP_FatElvis.Speed` (`self.Speed`) (`self.BP_FatElvis`))
  (`KismetSystemLibrary.K2_SetTimer` null "StopMoving" (`self.TimeAction`))
  (goto _label :!via `PlayFromStart`))

(event `StopMoving`
  (set `/Game/Character/BP_FatElvis.Speed` 0.0 (`self.BP_FatElvis`))
  (`KismetSystemLibrary.K2_SetTimer` null "ContinueMoving" (`self.TimeOpposition`))
  (goto _label :!via `Stop`))

(fn `UserConstructionScript`
  (`parent.UserConstructionScript`))