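; BP_NestElvis3 is a nest Blueprint that drives BPFatElvis back and forth along a timeline-based move.
; StartMoving plays Timeline3 from the start, then timers alternate ReverseMoving and ContinueMoving, flipping the timeline direction and Elvis's Speed sign.
; Timeline updates feed MoveTurtle.
; On finish, it clears the timer stored by ContinueMoving, zeroes Speed and calls ResetActivation.
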(event `ContinueMoving`
  (set `/Game/Character/BP_FatElvis.Speed` (`self.Speed`) (`self.BP_FatElvis`))
  (bind _returnvalue (`KismetSystemLibrary.K2_SetTimer` null "ReverseMoving" (`self.TimeAction`)))
  (bind (_direction _time) (`Timeline|Timeline3` :!label _label)
    (:`Update`
      (`self.MoveTurtle` _time))
    (:`Finished`
      (`KismetSystemLibrary.K2_ClearAndInvalidateTimerHandle` _returnvalue)
      (set `/Game/Character/BP_FatElvis.Speed` 0.0 (`self.BP_FatElvis`))
      (`self.ResetActivation`))))

(event `self.StartMoving`
  (set `/Game/Character/BP_FatElvis.Speed` (`self.Speed`) (`self.BP_FatElvis`))
  (`KismetSystemLibrary.K2_SetTimer` null "ReverseMoving" (`self.TimeAction`))
  (goto _label :!via `PlayFromStart`))

(event `ReverseMoving`
  (set `/Game/Character/BP_FatElvis.Speed` (* -1 (`self.Speed`)) (`self.BP_FatElvis`))
  (`KismetSystemLibrary.K2_SetTimer` null "ContinueMoving" (`self.TimeOpposition`))
  (goto _label :!via `Reverse`))

(fn `UserConstructionScript`
  (`parent.UserConstructionScript`))