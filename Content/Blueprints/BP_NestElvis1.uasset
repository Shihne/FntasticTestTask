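; BP_NestElvis1 is a nest variant that spawns and moves a BP_FatElvis turtle, building on its parent class.
; SpawnTurtle destroys any existing Elvis with destination Niagara and poof effects, then spawns a replacement at the nest with nest effects and stores it as the Turtle.
; StartMoving sets the turtle's speed and plays a timeline that drives MoveTurtle, then zeroes the speed and resets activation when finished.
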(event `self.StartMoving`
  (set `/Game/Character/BP_FatElvis.Speed` (`self.Speed`) (`self.BP_FatElvis`))
  (bind (_direction _time) (`Timeline|Timeline1` :!via `PlayFromStart`)
    (:`Update`
      (`self.MoveTurtle` _time))
    (:`Finished`
      (set `/Game/Character/BP_FatElvis.Speed` 0.0 (`self.BP_FatElvis`))
      (`self.ResetActivation`))))

(fn `SpawnTurtle`
  (`/Engine/EditorBlueprintResources/StandardMacros.IsValid` (`self.BP_FatElvis`)
    (:`Is Valid`
      (`ActorComponent.Activate` (`self.NiagaraDest`) true)
      (`ActorComponent.Activate` (`self.Poof`) true)
      (`self.K2_DestroyActor` (`self.BP_FatElvis`)))
    (:`Is Not Valid`
      _))
  (`ActorComponent.Activate` (`self.NiagaraNest`) true)
  (`ActorComponent.Activate` (`self.Poof`) true)
  (bind _returnvalue (`|SpawnActorFromClass` "/Game/Character/BP_FatElvis.BP_FatElvis_C" (`KismetMathLibrary.MakeTransform` (`self.K2_GetActorLocation` self)) "Undefined" "OverrideRootScale" null null))
  (bind _output_get (set `self.BP_FatElvis` _returnvalue))
  (set `self.Turtle` _output_get)
  (return))

(fn `UserConstructionScript`
  (`parent.UserConstructionScript`))