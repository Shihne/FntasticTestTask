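; Turtle nest actor that, when activated, spawns a BP_Turtle and moves it along a curved path to a Destination.
; A two-point spline, also built at construction, curves via CurvatureDegree tangents signed by the destination's relative position.
; A Timeline drives the turtle's XY and facing along the spline, keeping its Z.
; DoOnce blocks reactivation until movement finishes, each spawn replaces the previous turtle, and the scale-in timeline is unconnected.
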(event `NestActivation`
  (params (NewParam :type Boolean))
  (`/Engine/EditorBlueprintResources/StandardMacros.DoOnce` false :!label _label
    (:`Completed`
      (`self.SpawnTurtle`)
      (`self.BuildPath`)
      (`self.StartMoving`))))

(event `ResetActivation`
  (goto _label :!via `Reset`))

(event `StartMoving`
  (bind (_direction _time) (`Timeline|Timeline` :!via `PlayFromStart`)
    (:`Update`
      (`self.MoveTurtle` _time))
    (:`Finished`
      (`self.ResetActivation`))))

(fn `BuildPath`
  (bind _curvaturedegree (`self.CurvatureDegree`))
  (bind _returnvalue (* (`SceneComponent.GetRightVector` (`self.Destination`)) (* _curvaturedegree (`KismetMathLibrary.SignOfFloat` (- (.y (`SceneComponent.K2_GetComponentLocation` (`self.Destination`))) (.y (`SceneComponent.K2_GetComponentLocation` (`self.Nest`))))))))
  (bind _returnvalue_2 (* (`SceneComponent.GetForwardVector` (`self.Nest`)) (* (`KismetMathLibrary.SignOfFloat` (- (.x (`SceneComponent.K2_GetComponentLocation` (`self.Destination`))) (.x (`SceneComponent.K2_GetComponentLocation` (`self.Nest`))))) _curvaturedegree)))
  (`SplineComponent.ClearSplinePoints` (`self.Spline`) true)
  (`SplineComponent.AddSplinePoint` (`self.Spline`) (`SceneComponent.K2_GetComponentLocation` (`self.Nest`)) "World" true)
  (`SplineComponent.AddSplinePoint` (`self.Spline`) (`SceneComponent.K2_GetComponentLocation` (`self.Destination`)) "World" true)
  (`SplineComponent.SetTangentsAtSplinePoint` (`self.Spline`) 0 _returnvalue_2 _returnvalue_2 "World" true)
  (`SplineComponent.SetTangentsAtSplinePoint` (`self.Spline`) 1 _returnvalue _returnvalue "World" true))

(fn `MoveTurtle`
  (params (Time :type "Float (double-precision)"))
  (locals (MovingTime :type "Float (double-precision)"))
  (bind _spline (`self.Spline`))
  (bind _turtle (`self.Turtle`))
  (bind (_returnvalue_x _returnvalue_y _returnvalue_z) (`KismetMathLibrary.BreakVector` (`self.K2_GetActorLocation` _turtle)))
  (`self.K2_SetActorTransform` _turtle (`KismetMathLibrary.MakeTransform` (`KismetMathLibrary.MakeVector` (.x (`SplineComponent.GetLocationAtTime` _spline Time "World" false)) (.y (`SplineComponent.GetLocationAtTime` _spline Time "World" false)) _returnvalue_z) (`KismetMathLibrary.Conv_VectorToRotator` (`SplineComponent.GetDirectionAtTime` _spline Time "World" false))) false false))

(fn `SpawnTurtle`
  (bind _turtle (`self.Turtle`))
  (`/Engine/EditorBlueprintResources/StandardMacros.IsValid` _turtle
    (:`Is Valid`
      (`self.K2_DestroyActor` _turtle))
    (:`Is Not Valid`
      _))
  (bind _returnvalue (`|SpawnActorFromClass` "/Game/Blueprints/BP_Turtle.BP_Turtle_C" (`KismetMathLibrary.MakeTransform` (`self.K2_GetActorLocation` self)) "Undefined" "OverrideRootScale" null null))
  (set `self.Turtle` _returnvalue)
  (return))

(fn `UserConstructionScript`
  (`self.BuildPath`))