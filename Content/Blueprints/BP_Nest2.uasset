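; BP_Nest2 is a nest Blueprint that drives turtle movement in a stop-and-go rhythm.
; StartMoving plays a timeline from the start, feeding its track value to MoveTurtle on each update.
; Named timers alternate StopMoving and ContinueMoving, so movement runs for TimeAction, pauses for TimeOpposition, then resumes from where it stopped.
; When the timeline finishes, it calls ResetActivation.
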(event `ContinueMoving`
  (`KismetSystemLibrary.K2_SetTimer` null "StopMoving" (`self.TimeAction`))
  (bind (_direction _time) (`Timeline|Timeline2` :!label _label)
    (:`Update`
      (`self.MoveTurtle` _time))
    (:`Finished`
      (`self.ResetActivation`))))

(event `self.StartMoving`
  (`KismetSystemLibrary.K2_SetTimer` null "StopMoving" (`self.TimeAction`))
  (goto _label :!via `PlayFromStart`))

(event `StopMoving`
  (`KismetSystemLibrary.K2_SetTimer` null "ContinueMoving" (`self.TimeOpposition`))
  (goto _label :!via `Stop`))

(fn `UserConstructionScript`
  (`parent.UserConstructionScript`))