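; BP_Nest3 is a child nest Blueprint that moves a turtle back and forth along Timeline3, feeding its Time track into MoveTurtle.
; StartMoving plays from the start, then timers alternate ReverseMoving and ContinueMoving, using TimeAction for forward phases and TimeOpposition for reverse ones.
; When the timeline finishes, it clears the timer handle saved by ContinueMoving and calls ResetActivation.
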(event `ContinueMoving`
  (bind _returnvalue (`KismetSystemLibrary.K2_SetTimer` null "ReverseMoving" (`self.TimeAction`)))
  (bind (_direction _time) (`Timeline|Timeline3` :!label _label)
    (:`Update`
      (`self.MoveTurtle` _time))
    (:`Finished`
      (`KismetSystemLibrary.K2_ClearAndInvalidateTimerHandle` _returnvalue)
      (`self.ResetActivation`))))

(event `self.StartMoving`
  (`KismetSystemLibrary.K2_SetTimer` null "ReverseMoving" (`self.TimeAction`))
  (goto _label :!via `PlayFromStart`))

(event `ReverseMoving`
  (`KismetSystemLibrary.K2_SetTimer` null "ContinueMoving" (`self.TimeOpposition`))
  (goto _label :!via `Reverse`))

(fn `UserConstructionScript`
  (`parent.UserConstructionScript`))